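; VR pawn that controls a submarine through Oculus hand gestures.
; On BeginPlay it adds the gesture input mapping, sets floor tracking, binds both hands' recognition events and caches BP_Controller.
; Per-hand handlers map gesture names to controller calls for diving, rotation, movement, artefact and door interaction, and light missiles.
; Debug inputs record or delete gestures; releasing a record input can also stop rotation or movement, depending on the configured gesture name.
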(event Custom|CheckGestureR
  (params (GestureName :type String))
  (Development|PrintString GestureName true true "(R=0.000000,G=0.083861,B=1.000000,A=1.000000)")
  (switch string GestureName
    (:Pinkie_R
      (Default|SubMarineDiving (Variables|Default|GetAs%20BP%20Controller) 1.0))
    (:Nice_R
      (Default|SubMarineRotation (Variables|Default|GetAs%20BP%20Controller) 1.0))
    (:Ok_R
      (Default|CallArtefactInteraction (Variables|Default|GetAs%20BP%20Controller)))
    (:RockNRoll_R
      (Default|CallShootLightMissile (Variables|Default|GetAs%20BP%20Controller)))
    (:Pan_R
      (Default|SubMarineMovement (Variables|Default|GetAs%20BP%20Controller) 1.0))))

(event Custom|CheckGestureL
  (params (GestureName :type String))
  (Development|PrintString GestureName true true "(R=0.046600,G=1.000000,B=0.000000,A=1.000000)")
  (switch string GestureName
    (:Pinkie_L
      (Default|SubMarineDiving (Variables|Default|GetAs%20BP%20Controller) -1.0))
    (:Nice_L
      (Default|SubMarineRotation (Variables|Default|GetAs%20BP%20Controller) -1.0))
    (:Ok_L
      (Default|CallDoorInteraction (Variables|Default|GetAs%20BP%20Controller)))
    (:RockNRoll_L
      (Default|CallShootLightMissile (Variables|Default|GetAs%20BP%20Controller)))
    (:Pan_L
      (Default|SubMarineMovement (Variables|Default|GetAs%20BP%20Controller) 0.0))))

(event Input|EnhancedActionEvents|EnhancedInputActionIA_RGesture
  (params (ActionValue :type Boolean) (ElapsedSeconds :type Float%20%28double-precision%29) (TriggeredSeconds :type Float%20%28double-precision%29) (InputAction :type Input%20Action%20Object%20Reference :default "/Game/Team08Content/BP/Input/IA_RGesture.IA_RGesture"))
  ;[1 1 1] A Mettre à L & R (cutom pour le debug) + gesture Name à Changer à chaque gesture à enregistrer
  (:Started
    (Default|RecordGesture (Variables|Default|GetRightOculusHandGesture) (Variables|Default|GetGestureName_R))
    (Development|PrintString "RecordedRight"))
  (:Completed
    (switch string (Variables|Default|GetGestureName_R)
      (:Nice_R
        (Default|SubMarineStopRotation (Variables|Default|GetAs%20BP%20Controller)))
      (:Pan_R
        (Default|SubMarineStopMovement (Variables|Default|GetAs%20BP%20Controller))))))

(event Input|EnhancedActionEvents|EnhancedInputActionIA_LGesture
  (params (ActionValue :type Boolean) (ElapsedSeconds :type Float%20%28double-precision%29) (TriggeredSeconds :type Float%20%28double-precision%29) (InputAction :type Input%20Action%20Object%20Reference :default "/Game/Team08Content/BP/Input/IA_LGesture.IA_LGesture"))
  ;[1 1 1] A Mettre à L & R (cutom pour le debug) + gesture Name à Changer à chaque gesture à enregistrer
  (:Started
    (Default|RecordGesture (Variables|Default|GetLeftOculusHandGesture) (Variables|Default|GetGestureName_L))
    (Development|PrintString "RecordedLeft"))
  (:Completed
    (switch string (Variables|Default|GetGestureName_L)
      (:Nice_L
        (Default|SubMarineStopRotation (Variables|Default|GetAs%20BP%20Controller)))
      (:Pan_L
        (Default|SubMarineStopMovement (Variables|Default|GetAs%20BP%20Controller))))))

(event Input|EnhancedActionEvents|EnhancedInputActionIA_DeletGesture
  (params (ActionValue :type Boolean) (ElapsedSeconds :type Float%20%28double-precision%29) (TriggeredSeconds :type Float%20%28double-precision%29) (InputAction :type Input%20Action%20Object%20Reference :default "/Game/Team08Content/BP/Input/IA_DeletGesture.IA_DeletGesture"))
  (bind _gesturenametodelete (Variables|Default|GetGestureNameToDelete))
  ;[1 1 1] A Ajouter au DeleteInput (cutom pour le debug)
  (:Started
    (Default|DeleteGesture (Variables|Default|GetLeftOculusHandGesture) _gesturenametodelete)
    (Utilities|String|LogString _gesturenametodelete)))

(event EventBeginPlay
  (Input|AddMappingContext (PlayerController|LocalPlayerSubsystems|GetEnhancedInputLocalPlayerSubsystem (Game|GetPlayerController 0)) "/Game/Team08Content/BP/Input/IMC_CreateGesture.IMC_CreateGesture" 0 "(bIgnoreAllPressedKeysUntilRelease=True,bForceImmediately=False,bNotifyUserSettings=False)")
  (Class|HeadMountedDisplayFunctionLibrary|SetTrackingOrigin "Floor")
  (EventDispatchers|BindEventtoOnGestureRecognised (Variables|Default|GetRightOculusHandGesture) (EventDispatchers|CreateEvent :!event Custom|CheckGestureR))
  (EventDispatchers|BindEventtoOnGestureRecognised (Variables|Default|GetLeftOculusHandGesture) (EventDispatchers|CreateEvent :!event Custom|CheckGestureL))
  (bind _asbp_controller (Utilities|Casting|CastToBP_Controller (Pawn|GetController)))
  (Variables|Default|SetAs%20BP%20Controller _asbp_controller))

(fn ConstructionScript)