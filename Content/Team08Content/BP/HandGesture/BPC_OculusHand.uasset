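; Oculus hand component that records, deletes and recognises hand gestures.
; Gestures are named snapshots of component-space bone locations, persisted in a BP_SaveGameGesture slot and loaded at BeginPlay.
; A looping timer compares live bones to each saved gesture, taking the first with every bone within a distance threshold.
; Each match fires OnGestureRecognised with the name, repeating while held because the duplicate check is disconnected.
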(event Custom|DetectGestures
  ;[1 1 1] Call EventDispatcher If A Gesture Is Detected
  (bind (_result _gesture) (CallFunction|GetCurrentGesture))
  (if _result
    (bind _output_get (Variables|Default|SetCurrentGesture _gesture))
    (Default|CallOnGestureRecognised (.GestureName (Utilities|Struct|BreakS_Gesture _output_get)))))

(event EventBeginPlay
  (bind _output_get (Variables|Default|SetGesture (Variables|/Game/Team08Content/BP/HandGesture/BP_SaveGameGesture.BP_SaveGameGesture_C|GetGestures (CallFunction|LoadGestures))))
  (Utilities|Time|SetTimerbyEvent (delegate Custom|DetectGestures) (Variables|Default|GetRefreshRate) true)
  (for _array_element _output_get
    (Development|PrintString (.gesturename _array_element) true true "(R=0.203525,G=1.000000,B=0.197646,A=1.000000)" 1e+01)))

(fn LoadGestures
  (bind _returnvalue (SaveGame|DoesSaveGameExist (Variables|Default|GetGestureGameSlot)))
  (if _returnvalue
    (Development|PrintString "SAVE EXIST" true true "(R=1.000000,G=0.082829,B=0.000000,A=1.000000)")
    (bind _returnvalue_2 (SaveGame|LoadGamefromSlot (Variables|Default|GetGestureGameSlot)))
    (bind _asbp_save_game_gesture (Utilities|Casting|CastToBP_SaveGameGesture _returnvalue_2))
    (return _asbp_save_game_gesture)
    (else
      (Development|PrintString "SAVE DON'T EXIST" true true "(R=1.000000,G=0.000000,B=0.079394,A=1.000000)")
      (bind _returnvalue_3 (SaveGame|CreateSaveGameObject "/Game/Team08Content/BP/HandGesture/BP_SaveGameGesture.BP_SaveGameGesture_C"))
      (return _returnvalue_3))))

(fn RecordGesture
  (params (GestureName :type String))
  (bind _output_get (LocalVariables|SetGestureSaveGame (CallFunction|LoadGestures)))
  (if (not (CallFunction|DoesGestureExist? _output_get GestureName))
    (for _index (range 0 (- (Class|SkinnedMeshComponent|GetNumBones) 1))
      (bind _returnvalue (Class|PoseableMeshComponent|GetBoneLocationbyName (Class|SkinnedMeshComponent|GetBoneName _index) "ComponentSpace"))
      (Utilities|Array|Add (LocalVariables|GetBoneLocations) _returnvalue))
    (Utilities|Array|Add (Variables|/Game/Team08Content/BP/HandGesture/BP_SaveGameGesture.BP_SaveGameGesture_C|GetGestures (LocalVariables|GetGestureSaveGame)) (Utilities|Struct|MakeS_Gesture GestureName (LocalVariables|GetBoneLocations)))
    (SaveGame|SaveGametoSlot (LocalVariables|GetGestureSaveGame) (Variables|Default|GetGestureGameSlot))))

(fn DoesGestureExist?
  (params (SaveGameGesture :type BP%20Save%20Game%20Gesture%20Object%20Reference) (GestureName :type String))
  (Development|PrintString "Does Exist")
  (for _array_element (Variables|/Game/Team08Content/BP/HandGesture/BP_SaveGameGesture.BP_SaveGameGesture_C|GetGestures SaveGameGesture)
    (if (Utilities|Enum|Equal(Enum) (.GestureName (Utilities|Struct|BreakS_Gesture _array_element)) GestureName)
      (return true)))
  (return false))

(fn DeleteGesture
  (params (GestureName :type String))
  (bind _output_get (LocalVariables|SetGestureSaveGame (CallFunction|LoadGestures)))
  (for (_array_element _array_index) (Variables|/Game/Team08Content/BP/HandGesture/BP_SaveGameGesture.BP_SaveGameGesture_C|GetGestures _output_get)
    (if (== (.GestureName (Utilities|Struct|BreakS_Gesture _array_element)) GestureName)
      (LocalVariables|SetIndex _array_index)))
  (Utilities|Array|RemoveIndex (Variables|/Game/Team08Content/BP/HandGesture/BP_SaveGameGesture.BP_SaveGameGesture_C|GetGestures (LocalVariables|GetGestureSaveGame)) (LocalVariables|GetIndex))
  (SaveGame|SaveGametoSlot (LocalVariables|GetGestureSaveGame) (Variables|Default|GetGestureGameSlot)))

(fn GetCurrentGesture
  (for _array_element (Variables|Default|GetGesture)
    (for (_array_element_2 _array_index) (.BoneLocations (Utilities|Struct|BreakS_Gesture _array_element))
      (bind _returnvalue (Class|PoseableMeshComponent|GetBoneLocationbyName (Class|SkinnedMeshComponent|GetBoneName _array_index) "ComponentSpace"))
      (if (Variables|Default|GetDebug)
        (Development|PrintString (Utilities|String|ToString(Float) (Math|Float|Absolute(Float) (Math|Vector|VectorLength (- _returnvalue _array_element_2)))) true true "(R=0.000000,G=0.660000,B=1.000000,A=1.000000)" 0.0))
      (if (> (Math|Float|Absolute(Float) (Math|Vector|VectorLength (- _returnvalue _array_element_2))) (Variables|Default|GetTreshold))
        (LocalVariables|Setb_ValidGesture? false)))
    (if (LocalVariables|Getb_ValidGesture?)
      (return (LocalVariables|Getb_ValidGesture?) _array_element)
      (else
        (LocalVariables|Setb_ValidGesture? true))))
  (return false ""))

(fn EqualGesture
  (params (A :type S%20Gesture%20Structure) (B :type S%20Gesture%20Structure))
  (bind (_gesturename _bonelocations) (Utilities|Struct|BreakS_Gesture A))
  (bind (_gesturename_2 _bonelocations_2) (Utilities|Struct|BreakS_Gesture B))
  (return (and (Utilities|Enum|Equal(Enum) _gesturename _gesturename_2) (Utilities|Array|Identical _bonelocations _bonelocations_2))))