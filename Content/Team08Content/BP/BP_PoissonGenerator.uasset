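; BP_PoissonGenerator is a spawner actor that populates its location with batches of BP_PoissonB actors.
; It spawns a random-sized batch at BeginPlay, giving each actor a reference back to the generator and incrementing a running Count.
; When a BP_VRHandPawn stops overlapping it and Count is at or below a low threshold, it spawns another batch the same way.
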(event EventBeginPlay
  (for _index (range 0 (Math|Random|RandomIntegerinRange 20 30))
    (bind _returnvalue (Game|SpawnActorfromClass "/Game/Team08Content/BP/BP_PoissonB.BP_PoissonB_C" (Math|Transform|MakeTransform (Transformation|GetWorldLocation (Variables|Default|GetDefaultSceneRoot)) "0, 0, 0" "1.000000,1.000000,1.000000") "Undefined" "MultiplyWithRoot" 0 0))
    (Variables|/Game/Team08Content/BP/BP_PoissonB.BP_PoissonB_C|SetPoissonGenerator _returnvalue self)
    (CallFunction|Increment (Variables|Default|GetCount) 1)))

(event Collision|EventActorEndOverlap
  (params (OtherActor :type Actor%20Object%20Reference))
  (Utilities|Casting|CastToBP_VRHandPawn OtherActor)
  (if (<= (Variables|Default|GetCount) 10)
    (for _index (range 0 (Math|Random|RandomIntegerinRange 20 30))
      (bind _returnvalue (Game|SpawnActorfromClass "/Game/Team08Content/BP/BP_PoissonB.BP_PoissonB_C" (Math|Transform|MakeTransform (Transformation|GetWorldLocation (Variables|Default|GetDefaultSceneRoot)) "0, 0, 0" "1.000000,1.000000,1.000000") "Undefined" "MultiplyWithRoot" 0 0))
      (Variables|/Game/Team08Content/BP/BP_PoissonB.BP_PoissonB_C|SetPoissonGenerator _returnvalue self)
      (CallFunction|Increment (Variables|Default|GetCount) 1))))

(fn ConstructionScript)