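; Player controller for the VR submarine that handles shooting light missiles and interacting with doors and artefacts.
; On BeginPlay it binds three events to their handlers.
; The shot spawns BP_LightMissile at the submarine's LightMissileSpawn and sets its velocity from the camera's forward vector.
; Door and artefact interactions line trace forward from that same point on separate channels, with persistent debug drawing, and message hit actors implementing I_Interactable.
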(event Custom|SpawnLightMissile
  ;[1 0 0.1342] Shoot light missile
  (bind _asbp_vrsubmarine (Utilities|Casting|CastToBP_VRSubmarine (Pawn|GetControlledPawn (Game|GetPlayerController 0))))
  (bind _returnvalue (Game|SpawnActorfromClass "/Game/Team08Content/BP/BP_LightMissile.BP_LightMissile_C" (Math|Transform|MakeTransform (Transformation|GetWorldLocation (Variables|/Game/Team08Content/BP/BP_VRSubmarine.BP_VRSubmarine_C|GetLightMissileSpawn _asbp_vrsubmarine)) (Variables|/Script/Engine.SceneComponent|GetRelativeRotation (Variables|/Game/VRTemplate/Blueprints/VRPawn.VRPawn_C|GetCamera _asbp_vrsubmarine)) "1.000000,1.000000,1.000000") "Undefined" "MultiplyWithRoot" 0 0))
  (Game|Components|ProjectileMovement|SetVelocityinLocalSpace (Variables|/Game/Team08Content/BP/BP_LightMissile.BP_LightMissile_C|GetProjectileMovement _returnvalue) (* (Variables|/Game/Team08Content/BP/BP_LightMissile.BP_LightMissile_C|GetLightMissileSpeed _returnvalue) (Math|Vector|GetForwardVector (Variables|/Game/VRTemplate/Blueprints/VRPawn.VRPawn_C|GetCamera _asbp_vrsubmarine)))))

(event Custom|ArtefactLineTrace
  ;[1 0 0.1412] Interact with artefacts
  (bind _asbp_vrsubmarine (Utilities|Casting|CastToBP_VRSubmarine (Game|Player|GetPlayerPawn 0)))
  (bind _outhit (Collision|LineTraceByChannel (Transformation|GetWorldLocation (Variables|/Game/Team08Content/BP/BP_VRSubmarine.BP_VRSubmarine_C|GetLightMissileSpawn _asbp_vrsubmarine)) (+ (Transformation|GetWorldLocation (Variables|/Game/Team08Content/BP/BP_VRSubmarine.BP_VRSubmarine_C|GetLightMissileSpawn _asbp_vrsubmarine)) (* (Math|Vector|GetForwardVector (Transformation|GetWorldRotation (Variables|/Game/Team08Content/BP/BP_VRSubmarine.BP_VRSubmarine_C|GetLightMissileSpawn _asbp_vrsubmarine))) 1000)) "TraceTypeQuery5" false 0 "Persistent"))
  (if (Utilities|DoesObjectImplementInterface (.hitactor _outhit) "/Game/Team08Content/BP/Interfaces/I_Interactable.I_Interactable_C")
    (Class|IInteractable|Interact(Message) (.hitactor _outhit))))

(event Custom|DoorLineTrace
  ;[1 0 0.1412] Door line trace
  (bind _asbp_vrsubmarine (Utilities|Casting|CastToBP_VRSubmarine (Game|Player|GetPlayerPawn 0)))
  (bind _outhit (Collision|LineTraceByChannel (Transformation|GetWorldLocation (Variables|/Game/Team08Content/BP/BP_VRSubmarine.BP_VRSubmarine_C|GetLightMissileSpawn _asbp_vrsubmarine)) (+ (Transformation|GetWorldLocation (Variables|/Game/Team08Content/BP/BP_VRSubmarine.BP_VRSubmarine_C|GetLightMissileSpawn _asbp_vrsubmarine)) (* (Math|Vector|GetForwardVector (Transformation|GetWorldRotation (Variables|/Game/Team08Content/BP/BP_VRSubmarine.BP_VRSubmarine_C|GetLightMissileSpawn _asbp_vrsubmarine))) 1000)) "TraceTypeQuery4" false 0 "Persistent"))
  (if (Utilities|DoesObjectImplementInterface (.hitactor _outhit) "/Game/Team08Content/BP/Interfaces/I_Interactable.I_Interactable_C")
    (Class|IInteractable|Interact(Message) (.hitactor _outhit))))

(event EventBeginPlay
  ;[1 0 0.1342] Shoot light missile
  (EventDispatchers|BindEventtoShootLightMissile (delegate Custom|SpawnLightMissile))
  ;[1 0 0.1412] Door line trace
  (EventDispatchers|BindEventtoDoorInteraction (delegate Custom|DoorLineTrace))
  ;[1 0 0.1412] Interact with artefacts
  (EventDispatchers|BindEventtoArtefactInteraction (delegate Custom|ArtefactLineTrace)))

(fn ConstructionScript)