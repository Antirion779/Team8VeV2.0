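; Player controller for a VR submarine game, handling submarine driving, light missile fire and interaction with doors and artefacts.
; BeginPlay adds input mapping, attaches the hand pawn to the submarine, binds action events and starts a looping artefact-outline timer.
; Input drives the submarine's collision body with force and torque, zeroing velocities when input starts; the diving function is never called.
; Line traces from the pawn's raycast point message I_Interactable actors, using separate door and artefact channels.
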(event Custom|SpawnLightMissile
  ;[1 0 0.1342] Shoot light missile
  (bind _asbp_vrhand_pawn (Utilities|Casting|CastToBP_VRHandPawn (Pawn|GetControlledPawn (Game|GetPlayerController 0))))
  (bind _returnvalue (Game|SpawnActorfromClass "/Game/Team08Content/BP/BP_LightMissile.BP_LightMissile_C" (Math|Transform|MakeTransform (Transformation|GetWorldLocation (Variables|/Game/Team08Content/BP/HandGesture/BP_VRHandPawn.BP_VRHandPawn_C|GetRaycastSpawn _asbp_vrhand_pawn)) (Variables|/Script/Engine.SceneComponent|GetRelativeRotation (Variables|/Game/Team08Content/BP/HandGesture/BP_VRHandPawn.BP_VRHandPawn_C|GetCamera _asbp_vrhand_pawn)) "1.000000,1.000000,1.000000") "Undefined" "MultiplyWithRoot" 0 0))
  (Game|Components|ProjectileMovement|SetVelocityinLocalSpace (Variables|/Game/Team08Content/BP/BP_LightMissile.BP_LightMissile_C|GetProjectileMovement _returnvalue) (* (Variables|/Game/Team08Content/BP/BP_LightMissile.BP_LightMissile_C|GetLightMissileSpeed _returnvalue) (Math|Vector|GetForwardVector (Variables|/Game/Team08Content/BP/HandGesture/BP_VRHandPawn.BP_VRHandPawn_C|GetCamera _asbp_vrhand_pawn))))
  (Audio|PlaySound2D "/Game/Team08Content/Audio/RocketLaunchUnderWater.RocketLaunchUnderWater" 1.0 1.0 0.0 0 0))

(event Custom|ArtefactLineTrace
  ;[1 0 0.1412] Interact with artefacts
  (bind (_isinteractable _actor) (CallFunction|InteractableTrace "TraceTypeQuery4"))
  (if _isinteractable
    (Class|IInteractable|Interact(Message) _actor)))

(event Custom|DoorLineTrace
  ;[1 0 0.1412] Door line trace
  (bind (_isinteractable _actor) (CallFunction|InteractableTrace "TraceTypeQuery3"))
  (if _isinteractable
    (Class|IInteractable|Interact(Message) _actor)))

(event Custom|OutlineArtefact
  (bind _as_bp_vrhand_pawn (Variables|Default|GetAs%20BP%20VRHand%20Pawn))
  (bind _raycastspawn (Variables|/Game/Team08Content/BP/HandGesture/BP_VRHandPawn.BP_VRHandPawn_C|GetRaycastSpawn _as_bp_vrhand_pawn))
  (bind _returnvalue (Transformation|GetWorldLocation _raycastspawn))
  ;[1 0 0.1412] Interact with artefacts
  (bind _outhit (Collision|LineTraceByChannel _returnvalue (+ _returnvalue (* (Math|Vector|GetForwardVector (Transformation|GetWorldRotation _raycastspawn)) 1000)) "TraceTypeQuery4" false (Utilities|Array|MakeArray (Variables|Default|GetSubMarine)) "Persistent"))
  (if (Utilities|DoesObjectImplementInterface (.hitactor _outhit) "/Game/Team08Content/BP/Interfaces/I_Interactable.I_Interactable_C")
    (Class|IOutline|Outline(Message) (.hitactor _outhit))))

(event Input|EnhancedActionEvents|EnhancedInputActionIA_SubMarineMovement
  (params (ActionValue :type Vector :default "0, 0, 0") (ElapsedSeconds :type Float%20%28double-precision%29) (TriggeredSeconds :type Float%20%28double-precision%29) (InputAction :type Input%20Action%20Object%20Reference :default "/Game/Team08Content/Input/IA_SubMarineMovement.IA_SubMarineMovement"))
  ;[0 0 0] Sub Marine Move & Turn PC
  (:Triggered
    (CallFunction|SubMarineMovement (.y ActionValue))
    (CallFunction|SubMarineRotation (.x ActionValue)))
  (:Started
    (CallFunction|SubMarineStopMovement)
    (CallFunction|SubMarineStopRotation)))

(event EventBeginPlay
  (bind _returnvalue (PlayerController|LocalPlayerSubsystems|GetEnhancedInputLocalPlayerSubsystem))
  ;[0 0 0] IMC
  (Utilities|IsValid _returnvalue
    (:Is%20Valid
      (Input|AddMappingContext _returnvalue "/Game/VRTemplate/Input/IMC_Default.IMC_Default" 0 "(bIgnoreAllPressedKeysUntilRelease=True,bForceImmediately=False,bNotifyUserSettings=False)")
      (bind _asbp_vrhand_pawn (Utilities|Casting|CastToBP_VRHandPawn (Game|Player|GetPlayerPawn 0)))
      (bind _output_get (Variables|Default|SetAs%20BP%20VRHand%20Pawn _asbp_vrhand_pawn))
      (bind _returnvalue_2 (Actor|GetActorOfClass "/Game/Team08Content/BP/BP_SubMarine.BP_SubMarine_C"))
      (bind _output_get_2 (Variables|Default|SetSubMarine _returnvalue_2))
      (Transformation|AttachActorToActor _output_get _output_get_2 "None" "KeepWorld" "KeepWorld" "KeepWorld" true)
      ;[1 0 0.1342] Shoot light missile
      (EventDispatchers|BindEventtoShootLightMissile (delegate Custom|SpawnLightMissile))
      ;[1 0 0.1412] Door line trace
      (EventDispatchers|BindEventtoDoorInteraction (delegate Custom|DoorLineTrace))
      ;[1 0 0.1412] Interact with artefacts
      (EventDispatchers|BindEventtoArtefactInteraction (delegate Custom|ArtefactLineTrace))
      (Utilities|Time|SetTimerbyEvent (delegate Custom|OutlineArtefact) 0.1 true))))

(event EventTick
  (params (DeltaSeconds :type Float%20%28single-precision%29)))

(fn ConstructionScript)

(fn SubMarineMovement
  (params (Value :type Float%20%28double-precision%29))
  (bind _submarine (Variables|Default|GetSubMarine))
  (bind _submarine_bodycollision (Variables|/Game/Team08Content/BP/BP_SubMarine.BP_SubMarine_C|GetSubMarine_BodyCollision _submarine))
  (Physics|AddForce _submarine_bodycollision (* (Math|Vector|GetForwardVector _submarine_bodycollision) Value (Variables|Default|GetSpeed)) "None" true))

(fn SubMarineRotation
  (params (Value :type Float%20%28double-precision%29))
  (Class|PrimitiveComponent|AddTorqueinDegrees (Variables|/Game/Team08Content/BP/BP_SubMarine.BP_SubMarine_C|GetSubMarine_BodyCollision (Variables|Default|GetSubMarine)) (Math|Vector|MakeVector 0.0 0.0 (* Value (Variables|Default|GetRSpeed))) "None" true))

(fn SubMarineStopMovement
  (Physics|SetPhysicsLinearVelocity (Variables|/Game/Team08Content/BP/BP_SubMarine.BP_SubMarine_C|GetSubMarine_BodyCollision (Variables|Default|GetSubMarine)) "0, 0, 0" false "None"))

(fn SubMarineStopRotation
  (Class|PrimitiveComponent|SetPhysicsAngularVelocityinRadians (Variables|/Game/Team08Content/BP/BP_SubMarine.BP_SubMarine_C|GetSubMarine_BodyCollision (Variables|Default|GetSubMarine)) "0, 0, 0" false "None"))

(fn SubMarineDiving
  (params (Value :type Float%20%28double-precision%29))
  (bind _submarine (Variables|Default|GetSubMarine))
  (bind _submarine_bodycollision (Variables|/Game/Team08Content/BP/BP_SubMarine.BP_SubMarine_C|GetSubMarine_BodyCollision _submarine))
  (Physics|AddForce _submarine_bodycollision (* (Math|Vector|GetUpVector _submarine_bodycollision) Value (Variables|Default|GetRSpeed)) "None" true))

(fn InteractableTrace
  (params (TraceChannel :type ETraceTypeQuery%20Enum :default "TraceTypeQuery1"))
  (bind _as_bp_vrhand_pawn (Variables|Default|GetAs%20BP%20VRHand%20Pawn))
  (bind _raycastspawn (Variables|/Game/Team08Content/BP/HandGesture/BP_VRHandPawn.BP_VRHandPawn_C|GetRaycastSpawn _as_bp_vrhand_pawn))
  (bind _returnvalue (Transformation|GetWorldLocation _raycastspawn))
  (bind _outhit (Collision|LineTraceByChannel _returnvalue (+ _returnvalue (* (Math|Vector|GetForwardVector (Transformation|GetWorldRotation _raycastspawn)) 1000)) TraceChannel false (Utilities|Array|MakeArray (Variables|Default|GetSubMarine)) "Persistent"))
  (if (Utilities|DoesObjectImplementInterface (.hitactor _outhit) "/Game/Team08Content/BP/Interfaces/I_Interactable.I_Interactable_C")
    (return (Utilities|DoesObjectImplementInterface (.hitactor _outhit) "/Game/Team08Content/BP/Interfaces/I_Interactable.I_Interactable_C") (.hitactor _outhit))))