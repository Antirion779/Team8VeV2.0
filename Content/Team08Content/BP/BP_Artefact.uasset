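; BP_Artefact is a collectible artefact, one of three set by ArtefactNumber, which selects its mesh and vertical offset on BeginPlay.
; A billboard pivot turns toward the player camera every tick, and overlap with the VR hand pawn plays a cursor sound.
; Interact notifies BP_GameManager which artefact was collected, then destroys the actor.
; Outline alternately shows the outline mesh or hides it after a short delay.
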(event OnComponentBeginOverlap(Sphere)
  (params (OverlappedComponent :type Primitive%20Component%20Object%20Reference) (OtherActor :type Actor%20Object%20Reference) (OtherComp :type Primitive%20Component%20Object%20Reference) (OtherBodyIndex :type Integer) (bFromSweep :type Boolean) (SweepResult :type Hit%20Result%20Structure%20%28by%20ref%29))
  (Utilities|Casting|CastToBP_VRHandPawn OtherActor)
  (Audio|PlaySound2D "/Game/Team08Content/Audio/CursorApparait.CursorApparait" 1.0 1.0 0.0 0 0))

(event EventTick
  (params (DeltaSeconds :type Float%20%28single-precision%29))
  (bind _billboardpivot (Variables|Default|GetBillboardPivot))
  (Transformation|SetWorldRotation _billboardpivot (Math|Rotator|FindLookatRotation (Transformation|GetWorldLocation _billboardpivot) (Transformation|GetActorLocation (Game|GetPlayerCameraManager 0))) false false))

(event EventOutline
  (if (Variables|Default|GetActiveOutline)
    (Utilities|FlowControl|Delay 1.0)
    (Rendering|SetVisibility (Variables|Default|GetCubeOutline) false false)
    (Variables|Default|SetActiveOutline false)
    (else
      (Variables|Default|SetActiveOutline true)
      (Rendering|SetVisibility (Variables|Default|GetCubeOutline) true false))))

(event EventBeginPlay
  (bind _artefactnumber (Variables|Default|GetArtefactNumber))
  (bind _returnvalue (- _artefactnumber 1))
  (Components|StaticMesh|SetStaticMesh (Variables|Default|GetCube) (Utilities|Array|Get(acopy) (Variables|Default|GetSMs) _returnvalue))
  (Transformation|AddRelativeLocation (Variables|Default|GetCube) (Math|Vector|MakeVector 0.0 0.0 (* _returnvalue (Variables|Default|GetOffset))) false false))

(event EventInteract
  (bind _returnvalue (Actor|GetActorOfClass "/Game/Team08Content/BP/BP_GameManager.BP_GameManager_C"))
  (switch int (Variables|Default|GetArtefactNumber)
    (:1
      (Default|GetFirstArtefact _returnvalue))
    (:2
      (Default|GetSecondArtefact _returnvalue))
    (:3
      (Default|GetThirdArtefact _returnvalue)))
  (Actor|DestroyActor))

(fn ConstructionScript)