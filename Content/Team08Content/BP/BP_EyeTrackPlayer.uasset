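; BP_EyeTrackPlayer is an actor whose eyeball turns to face the VR player while they are within range.
; It caches BP_Controller on BeginPlay to reach the VR hand pawn.
; Entering the EyeTrackingLimit volume starts a looping timer that snaps the Eyeball's world rotation toward that pawn's location, avoiding Tick.
; Leaving the volume clears the timer, so tracking stops.
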(event OnComponentBeginOverlap(EyeTrackingLimit)
  (params (OverlappedComponent :type Primitive%20Component%20Object%20Reference) (OtherActor :type Actor%20Object%20Reference) (OtherComp :type Primitive%20Component%20Object%20Reference) (OtherBodyIndex :type Integer) (bFromSweep :type Boolean) (SweepResult :type Hit%20Result%20Structure%20%28by%20ref%29))
  (Utilities|Casting|CastToBP_Controller (Game|GetInstigatorController OtherActor))
  (bind _returnvalue (Utilities|Time|SetTimerbyEvent (delegate Custom|TrackPlayer) 0.1 true))
  (Variables|Default|SetTimer _returnvalue))

(event OnComponentEndOverlap(EyeTrackingLimit)
  (params (OverlappedComponent :type Primitive%20Component%20Object%20Reference) (OtherActor :type Actor%20Object%20Reference) (OtherComp :type Primitive%20Component%20Object%20Reference) (OtherBodyIndex :type Integer))
  (Utilities|Casting|CastToBP_Controller (Game|GetInstigatorController OtherActor))
  (if (Class|KismetSystemLibrary|TimerExistsHandle (Variables|Default|GetTimer))
    (Utilities|Time|ClearandInvalidateTimerbyHandle (Variables|Default|GetTimer))))

(event Custom|TrackPlayer
  (bind _playercontroller (Variables|Default|GetPlayerController))
  (bind _eyeball (Variables|Default|GetEyeball))
  (bind _returnvalue (Transformation|GetWorldLocation _eyeball))
  (bind _as_bp_vrhand_pawn (Variables|/Game/Team08Content/BP/BP_Controller.BP_Controller_C|GetAs%20BP%20VRHand%20Pawn _playercontroller))
  (bind _returnvalue_2 (Transformation|GetActorLocation _as_bp_vrhand_pawn))
  (bind _returnvalue_3 (Math|Rotator|FindLookatRotation _returnvalue _returnvalue_2))
  (Transformation|SetWorldRotation (Variables|Default|GetEyeball) (Math|Rotator|MakeRotator (.roll _returnvalue_3) (.pitch _returnvalue_3) (.yaw _returnvalue_3)) false false))

(event EventBeginPlay
  (bind _asbp_controller (Utilities|Casting|CastToBP_Controller (Game|GetPlayerController 0)))
  (Variables|Default|SetPlayerController _asbp_controller))

(event Collision|EventActorBeginOverlap
  (params (OtherActor :type Actor%20Object%20Reference)))

(event EventTick
  (params (DeltaSeconds :type Float%20%28single-precision%29)))

(fn ConstructionScript)