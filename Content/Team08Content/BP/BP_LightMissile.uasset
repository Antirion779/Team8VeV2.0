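; BP_LightMissile is a light-emitting projectile that bursts into a wide illuminating flash on impact, apparently underwater given its explosion sound.
; When its collision component is hit, it hides the sphere mesh, sets the point light's intensity and widens its radius, and plays the sound at the sphere's location.
; A timeline then scales the light's intensity along a fade track and destroys the actor when it finishes.
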(event OnComponentHit(Collision)
  (params (HitComponent :type Primitive%20Component%20Object%20Reference) (OtherActor :type Actor%20Object%20Reference) (OtherComp :type Primitive%20Component%20Object%20Reference) (NormalImpulse :type Vector :default "0, 0, 0") (Hit :type Hit%20Result%20Structure%20%28by%20ref%29))
  (bind _pointlight (Variables|Default|GetPointLight))
  (Rendering|SetVisibility (Variables|Default|GetSphere) false false)
  (Rendering|Components|Light|SetIntensity _pointlight (Variables|Default|GetLightIntensity))
  (Rendering|Lighting|SetAttenuationRadius _pointlight 5e+03)
  (Audio|PlaySoundatLocation "/Game/Team08Content/Audio/ExplosionRocketLightUnderWater.ExplosionRocketLightUnderWater" (Transformation|GetWorldLocation (Variables|Default|GetSphere)) "0, 0, 0" 1.0 1.0 0.0 0 0 0 0)
  (bind _fadetrack (Timeline|Timeline Play)
    (:Update
      (Rendering|Components|Light|SetIntensity (Variables|Default|GetPointLight) (* _fadetrack (Variables|Default|GetLightIntensity))))
    (:Finished
      (Actor|DestroyActor))))

(fn ConstructionScript)