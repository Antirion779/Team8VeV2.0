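; BP_GameManager tracks which of three artefacts have been found and updates the artefact HUD to match.
; On BeginPlay it finds the BP_ArtefactHUD actor and caches its W_ArtefactHUD widget.
; Separate events for the first, second and third artefact each set a found flag and make the matching fill image fully opaque.
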(event Custom|GetSecondArtefact
  (Variables|Default|SetSecondArtefactFound true)
  (Class|Image|SetOpacity (Variables|/Game/Team08Content/UMG/W_ArtefactHUD.W_ArtefactHUD_C|GetFill_1 (Variables|Default|GetAs%20W%20Artefact%20HUD)) 1.0))

(event Custom|GetFirstArtefact
  (Variables|Default|SetFirstArtefactFound true)
  (Class|Image|SetOpacity (Variables|/Game/Team08Content/UMG/W_ArtefactHUD.W_ArtefactHUD_C|GetFill (Variables|Default|GetAs%20W%20Artefact%20HUD)) 1.0))

(event Custom|GetThirdArtefact
  (Variables|Default|SetThirdArtefactFound true)
  (Class|Image|SetOpacity (Variables|/Game/Team08Content/UMG/W_ArtefactHUD.W_ArtefactHUD_C|GetFill_2 (Variables|Default|GetAs%20W%20Artefact%20HUD)) 1.0))

(event EventBeginPlay
  (bind _returnvalue (Actor|GetActorOfClass "/Game/Team08Content/BP/HUD/BP_ArtefactHUD.BP_ArtefactHUD_C"))
  (bind _asw_artefact_hud (Utilities|Casting|CastToW_ArtefactHUD (UserInterface|GetWidget (Variables|/Game/Team08Content/BP/HUD/BP_ArtefactHUD.BP_ArtefactHUD_C|GetWidget _returnvalue))))
  (Variables|Default|SetAs%20W%20Artefact%20HUD _asw_artefact_hud))

(fn ConstructionScript)